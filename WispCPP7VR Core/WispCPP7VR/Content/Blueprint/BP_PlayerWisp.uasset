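; BP_PlayerWisp is a wisp actor, apparently the player's, that tracks the actor it senses.
; On BeginPlay it binds to OnActorSensed and stores each reported actor in SensedActor.
; Its interaction functions are stubs: CanInteract returns false, name and hint are empty, and hover and interact events do nothing.
; Disconnected nodes hold unfinished interaction calls and debug prints that never run.
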(event `self.ReceiveBeginPlay`
  (add `self.OnActorSensed` (delegate `OnActorSensed_Event`)))

(event `self.ReceiveActorBeginOverlap`
  (params (OtherActor :type "Actor Object Reference")))

(event `InteractionInterface.OnBeginHover`)

(event `InteractionInterface.OnEndHover`)

(event `InteractionInterface.OnInteract`
  (params (Interactor :type "Actor Object Reference")))

(event `InteractionInterface.OnSecondaryInteract`
  (params (Interactor :type "Actor Object Reference")))

(event `OnActorSensed_Event` :!signature `self.OnActorSensed`
  (params (SensedActor :type "Actor Object Reference"))
  (set `self.SensedActor` SensedActor))

(fn `CanInteract`
  (params (Interactor :type "Actor Object Reference"))
  (returns (ReturnValue :type Boolean))
  (return false))

(fn `GetInteractableName`
  (returns (ReturnValue :type Text))
  (return ""))

(fn `GetInteractionHint`
  (returns (ReturnValue :type String))
  (return ""))

(fn `UserConstructionScript`)